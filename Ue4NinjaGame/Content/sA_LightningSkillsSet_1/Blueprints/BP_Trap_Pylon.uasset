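; BP_Trap_Pylon is a lightning trap pylon actor that periodically fires an attack effect while it is not idle.
; Each Tick, a set Attack flag activates the AttackFx component without resetting it, then clears itself.
; A second Tick branch re-arms the flag through a Delay of AttackDelay, forming a repeating timer.
; The graph handles only the effect timing, with no overlap or damage logic.
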(event EventBeginPlay)

(event Collision|EventActorBeginOverlap
  (params (OtherActor :type Actor%20Object%20Reference)))

(event EventTick
  (params (DeltaSeconds :type Float%20%28single-precision%29))
  (Utilities|FlowControl|Sequence
    (:then_0
      (if (not (Variables|Default|GetIdle))
        (if (Variables|Default|GetAttack)
          (Components|Activation|SetActive (Variables|Default|GetAttackFx) true false)
          (Variables|Default|SetAttack false))))
    (:then_1
      (if (not (Variables|Default|GetIdle))
        (Utilities|FlowControl|Delay (Variables|Default|GetAttackDelay))
        (Variables|Default|SetAttack true)))))

(fn ConstructionScript)