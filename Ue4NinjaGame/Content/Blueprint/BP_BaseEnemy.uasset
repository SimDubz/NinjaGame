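; Base enemy character that chases the player, optionally melees on arrival, and awards score on death.
; Data table stats drive speed, combat and health, which scales with game time at spawn and is hinted by attached horns cycling per increase.
; AI move, attack and recovery loop back into the chase.
; Hits update a crack material and branch into base, stun or recursively ticking poison, which deals a percentage of spawn health.
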(event Custom|MoveTo
  (bind _returnvalue (Game|Player|GetPlayerPawn 0))
  ;[1 1 1] Move to logic
  (Variables|/Game/Monster/Animation/AnimBP_Monster.AnimBP_Monster_C|SetMoving (Variables|Default|GetAnimInstance) true)
  (AI|AIMoveTo self (Transformation|GetActorLocation _returnvalue) _returnvalue 0.0 false
    (:OnSuccess
      (Utilities|AttackLogic))
    (:OnFail
      (Variables|/Game/Monster/Animation/AnimBP_Monster.AnimBP_Monster_C|SetMoving (Variables|Default|GetAnimInstance) false))))

(event Custom|ApplyPoisonDamage
  (bind _poisonticknumber (Variables|Default|GetPoisonTickNumber))
  ;[1 1 1] Posion event
  (bind _returnvalue (Utilities|GetDataTableRow "/Game/Blueprint/Stats_DataTable.Stats_DataTable" "ShurikenPoisonTickTime")
    (:then
      (Utilities|FlowControl|Delay (.value _returnvalue))
      (bind _returnvalue_2 (Utilities|GetDataTableRow "/Game/Blueprint/Stats_DataTable.Stats_DataTable" "ShurikenPoisonPercentage")
        (:then
          (CallFunction|DmgInput (* (.value _returnvalue_2) (Variables|Default|GetNormalEnemyHealth)) "NewEnumerator0")
          (Math|Integer|DecrementInt _poisonticknumber
            (:%20%20
              (if (!= _poisonticknumber 0)
                (Variables|Default|SetHitEmitter "/Game/Marketplace/Stylized_VFX_StPack/Particles/UPDATE_1_3/P_Web_Hit_01_Poison.P_Web_Hit_01_Poison")
                (CallFunction|ApplyPoisonDamage)))))))))

(event Custom|DestroyAfterDelay
  (params (DelayTime :type Float%20%28single-precision%29))
  ;[1 1 1] Delay before destroy to make sure we have time to run code
  (Utilities|FlowControl|Delay DelayTime)
  (Actor|DestroyActor))

(event Custom|Recovered
  ;[1 1 1] Receive dmg
  (CallFunction|Moveto))

(event EventBeginPlay
  ;[1 1 1] Begin play
  (bind _asanim_bp_monster (Utilities|Casting|CastToAnimBP_Monster (Components|SkeletalMesh|GetAnimInstance (Variables|Character|GetMesh))))
  (Variables|Default|SetAnimInstance _asanim_bp_monster)
  (CallFunction|Moveto))

(event EventDmgInput
  (params (Damages :type Float%20%28single-precision%29) (AttackType :type EShurikenEffects%20Enum :default "NewEnumerator0"))
  ;[1 1 1] Receive dmg
  (Utilities|OnHitLogic Damages AttackType))

(fn ConstructionScript
  ;[1 1 1] Base Health calculation
  (bind _returnvalue (CallFunction|BaseHealthMath))
  (Variables|Default|SetHealth _returnvalue)
  (Variables|Default|SetBaseHealth _returnvalue)
  (bind _returnvalue_2 (Utilities|GetDataTableRow "/Game/Blueprint/Stats_DataTable.Stats_DataTable" "EnemyBaseSpeed")
    (:then
      (Variables|/Script/Engine.CharacterMovementComponent|SetMaxWalkSpeed (Variables|Character|GetCharacterMovement) (.value _returnvalue_2))
      ;[1 1 1] Add horns based on health increase rate
      (bind _returnvalue_3 (Utilities|GetDataTableRow "/Game/Blueprint/Stats_DataTable.Stats_DataTable" "EnemyHealthIncreaseRate")
        (:then
          (if (!= (- (/ (Math|Float|Round (Utilities|Time|GetTimeSeconds)) (Math|Float|Truncate (.value _returnvalue_3))) (* (/ (/ (Math|Float|Round (Utilities|Time|GetTimeSeconds)) (Math|Float|Truncate (.value _returnvalue_3))) 5) 5)) 0)
            (for _index (range 1 (- (/ (Math|Float|Round (Utilities|Time|GetTimeSeconds)) (Math|Float|Truncate (.value _returnvalue_3))) (* (/ (/ (Math|Float|Round (Utilities|Time|GetTimeSeconds)) (Math|Float|Truncate (.value _returnvalue_3))) 5) 5)))
              (Transformation|AttachComponentToComponent (Utilities|Select :Index _index :Option%200 0 :Option%201 (Variables|Default|GetHorn_1) :Option%202 (Variables|Default|GetHorn_2) :Option%203 (Variables|Default|GetHorn_3) :Option%204 (Variables|Default|GetHorn_4) :Option%205 0) (Variables|Character|GetMesh) (Utilities|Select :Index _index :Option%200 "None" :Option%201 "Horn_1" :Option%202 "Horn_2" :Option%203 "Horn_3" :Option%204 "Horn_4" :Option%205 "None") "SnapToTarget" "SnapToTarget" "SnapToTarget" true))))))))

(fn Death
  (bind _capsulecomponent (Variables|Collision|GetCapsuleComponent))
  ;[1 1 1] Death
  (bind _asbp_base_pawn (Utilities|Casting|CastToBP_BasePawn (Game|Player|GetPlayerPawn 0)))
  (bind _returnvalue (Utilities|GetDataTableRow "/Game/Blueprint/Stats_DataTable.Stats_DataTable" "EnemyBasePoints")
    (:then
      (Default|UpdateScore _asbp_base_pawn (Math|Float|Truncate (* (.value _returnvalue) (Variables|Default|GetScoreMultiplier))))
      (Effects|SpawnEmitteratLocation "/Game/Marketplace/AdvancedMagicFX12/particles/P_ky_hit_dark.P_ky_hit_dark" (Transformation|GetWorldLocation _capsulecomponent) "0, 0, 0" (* (Transformation|GetWorldScale _capsulecomponent) 0.75))
      (CallFunction|LogiconDestroy)
      (return))))

(fn LogiconDestroy
  (CallFunction|DestroyAfterDelay 0.0))

(fn BaseHealthMath
  (bind _returnvalue (Utilities|GetDataTableRow "/Game/Blueprint/Stats_DataTable.Stats_DataTable" "EnemyHealthIncreaseRate")
    (:then
      (bind _returnvalue_2 (Utilities|GetDataTableRow "/Game/Blueprint/Stats_DataTable.Stats_DataTable" "EnemyHealthIncrease%")
        (:then
          (bind _returnvalue_3 (Utilities|GetDataTableRow "/Game/Blueprint/Stats_DataTable.Stats_DataTable" "EnemyBaseHealth")
            (:then
              (Variables|Default|SetNormalEnemyHealth (* (.value _returnvalue_3) (+ (* (/ (Math|Float|Round (Utilities|Time|GetTimeSeconds)) (Math|Float|Truncate (.value _returnvalue))) (.value _returnvalue_2)) 1.0)))
              (return (* (.value _returnvalue_3) (+ (* (/ (Math|Float|Round (Utilities|Time|GetTimeSeconds)) (Math|Float|Truncate (.value _returnvalue))) (.value _returnvalue_2)) 1.0))))))))))