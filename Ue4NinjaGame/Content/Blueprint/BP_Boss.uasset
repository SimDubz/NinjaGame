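; Boss enemy that extends a parent enemy with a ranged attack, boosted health, a score multiplier and extra loot.
; When a BP_BasePawn is inside AttackSphere, it halts, turns toward the player via a timeline, fires a projectile after a wind-up, resumes moving, then retries after cooldown.
; On death it spawns random ability pickups at offsets plus a heart pickup.
; Timings, multipliers and drop count come from a stats DataTable.
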(event OnComponentBeginOverlap(AttackSphere)
  (params (OverlappedComponent :type Primitive%20Component%20Object%20Reference) (OtherActor :type Actor%20Object%20Reference) (OtherComp :type Primitive%20Component%20Object%20Reference) (OtherBodyIndex :type Integer) (bFromSweep :type Boolean) (SweepResult :type Hit%20Result%20Structure%20%28by%20ref%29))
  ;[1 1 1] On overlap AttackShpere
  (CallFunction|ShootProjectile))

(event Custom|StartLookAtPlayer
  ;[1 1 1] Look at player
  (Timeline|LookAtPlayer Play
    (:Update
      (Transformation|SetActorRotation (Math|Rotator|MakeRotator 0.0 0.0 (.yaw (Math|Rotator|FindLookatRotation (Transformation|GetWorldLocation (Variables|Default|GetCapsuleComponent)) (Transformation|GetActorLocation (Game|Player|GetPlayerPawn 0)))))))))

(event Custom|StopLookAtPlayer
  ;[1 1 1] Look at player
  (Timeline|LookAtPlayer Stop
    (:Update
      (Transformation|SetActorRotation (Math|Rotator|MakeRotator 0.0 0.0 (.yaw (Math|Rotator|FindLookatRotation (Transformation|GetWorldLocation (Variables|Default|GetCapsuleComponent)) (Transformation|GetActorLocation (Game|Player|GetPlayerPawn 0)))))))))

(event Custom|ShootProjectile
  (bind _projectilespawnlocation (Variables|Default|GetProjectileSpawnLocation))
  (bind _returnvalue (Transformation|GetWorldTransform _projectilespawnlocation))
  ;[1 1 1] Shoot Projectile
  (if (and (> (Utilities|Array|Length (Collision|GetOverlappingActors (Variables|Default|GetAttackSphere) "/Game/Blueprint/BP_BasePawn.BP_BasePawn_C" :!class /Script/Engine.PrimitiveComponent)) 0) (not (Variables|Default|GetInCooldown)))
    (Variables|/Game/Monster/Animation/AnimBP_Monster.AnimBP_Monster_C|SetMoving (Variables|Default|GetAnimInstance) false)
    (Class|NavMovementComponent|StopActiveMovement (Variables|Character|GetCharacterMovement))
    (Variables|Default|SetInCooldown true)
    (Variables|/Game/Monster/Animation/AnimBP_Monster.AnimBP_Monster_C|SetAttacking (Variables|Default|GetAnimInstance) true)
    (CallFunction|StartLookatPlayer)
    (Audio|PlaySoundatLocation "/Game/Ultimate_SFX_Bundle/Monster_Sounds_Pro/Wavs/Huge_monster_attack/Huge_monster_attack_3.Huge_monster_attack_3" (Transformation|GetWorldLocation (Variables|Default|GetCapsuleComponent)) "0, 0, 0" 1.0 1.0 0.0 0 0 0) ; Shoot sound
    (bind _returnvalue_2 (Utilities|GetDataTableRow "/Game/Blueprint/Stats_DataTable.Stats_DataTable" "EnemyAttackTime")
      (:then
        (Utilities|FlowControl|Delay (.value _returnvalue_2)) ; Time of attack
        (Game|SpawnActorfromClass "/Game/Blueprint/BP_BossProjectile.BP_BossProjectile_C" (Math|Transform|MakeTransform (.location _returnvalue) (.rotation _returnvalue) "1,1,1") "Undefined" 0 0)
        (CallFunction|StopLookatPlayer)
        (CallFunction|Moveto)
        (bind _returnvalue_3 (Utilities|GetDataTableRow "/Game/Blueprint/Stats_DataTable.Stats_DataTable" "BossAbilityCooldown")
          (:then
            (Utilities|FlowControl|Delay (.value _returnvalue_3)) ; Next shot cooldown
            (Variables|Default|SetInCooldown false)
            (CallFunction|ShootProjectile)))))))

(event EventBeginPlay
  (|CallParentFunction))

(event Collision|EventActorBeginOverlap
  (params (OtherActor :type Actor%20Object%20Reference)))

(fn ConstructionScript
  (|CallParentFunction)
  (bind _returnvalue (Utilities|GetDataTableRow "/Game/Blueprint/Stats_DataTable.Stats_DataTable" "BossScoreMultiplier")
    (:then
      (Variables|Default|SetScoreMultiplier (.value _returnvalue))
      (Variables|Default|SetDeathSounds (Utilities|Array|MakeArray "/Game/Ultimate_SFX_Bundle/Monster_Sounds_Pro/Wavs/Huge_monster_Death/Huge_monster_Death_1.Huge_monster_Death_1")))))

(fn LogiconDestroy
  (bind _mesh (Variables|Character|GetMesh))
  (bind _returnvalue (Transformation|GetWorldLocation _mesh))
  ;[1 1 1] Spawn Abilities
  (bind _returnvalue_2 (Utilities|GetDataTableRow "/Game/Blueprint/Stats_DataTable.Stats_DataTable" "BossAbilitySpawnNumber")
    (:then
      (for _index (range 1 (Math|Float|Truncate (.value _returnvalue_2)))
        (Game|SpawnActorfromClass "/Game/Blueprint/AltShurikens/BP_AbilityPickup_Random.BP_AbilityPickup_Random_C" (Math|Transform|MakeTransform (+ _returnvalue (Utilities|Select :Index _index :Option%200 "0, 0, 0" :Option%201 "250.000000, 0, 0" :Option%202 "-250.000000, 0, 0" :Option%203 "0,-250.000000, 0")) "0, 0, 0" "1,1,1") "Undefined" 0 0))
      (Game|SpawnActorfromClass "/Game/Blueprint/AltShurikens/BP_HeartPickup.BP_HeartPickup_C" (Math|Transform|MakeTransform _returnvalue "0, 0, 0" "1,1,1") "Undefined" 0 0)
      (|CallParentFunction)
      (return))))

(fn BaseHealthMath
  (bind _returnvalue (|CallParentFunction))
  (bind _returnvalue_2 (Utilities|GetDataTableRow "/Game/Blueprint/Stats_DataTable.Stats_DataTable" "BossHealthMultiplier")
    (:then
      (return (* _returnvalue (.value _returnvalue_2))))))