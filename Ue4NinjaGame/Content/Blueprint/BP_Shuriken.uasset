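; Shuriken projectile that damages enemies, with lifespan, speed, size and base damage read from a stats DataTable.
; Its Effects list toggles behaviors delegated to components: Big and Multiple at spawn, Stun, Ricochet, Poison and Explosion on impact.
; Pawn capsule overlaps send damage through BPI_Damage, doubled for Big, and record victims so pierce hits each once.
; Actor hits can trigger Explosion and always destroy it; enemy overlaps destroy it unless piercing.
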(event Custom|Hit
  (params (SelfActor :type Actor%20Object%20Reference) (OtherActor :type Actor%20Object%20Reference) (NormalImpulse :type Vector) (Hit :type Hit%20Result%20Structure%20%28by%20ref%29))
  ;[1 1 1] On Hit Event
  (CallFunction|BeforeDestroyOntHit OtherActor Hit)
  (CallFunction|DestroyLogic true))

(event Custom|Overlapped
  (params (OverlappedComponent :type Primitive%20Component%20Object%20Reference) (OtherActor :type Actor%20Object%20Reference) (OtherComp :type Primitive%20Component%20Object%20Reference) (OtherBodyIndex :type Integer) (bFromSweep :type Boolean) (SweepResult :type Hit%20Result%20Structure%20%28by%20ref%29))
  (bind _hittedmonster (Variables|Default|GetHittedMonster))
  ;[1 1 1] On overlap event
  (bind _ascapsule_collision (Utilities|Casting|CastToCapsuleComponent OtherComp))
  (if (Math|Boolean|ANDBoolean (Utilities|Enum|Equal(Enum) (Collision|GetCollisionObjectType _ascapsule_collision) "ECC_Pawn") (Utilities|DoesObjectImplementInterface OtherActor "/Game/Blueprint/BPI_Damage.BPI_Damage_C") (not (Utilities|Array|ContainsItem (Variables|Default|GetHittedMonster) OtherActor)))
    ;;[1 0.1771 0.1771] main use for the pierce
    (if (not (Utilities|Array|ContainsItem _hittedmonster OtherActor))
      (Utilities|Array|AddUnique _hittedmonster OtherActor)
      (CallFunction|BeforeDestroyonEnemy OtherActor)
      (CallFunction|DestroyLogic false))))

(event EventBeginPlay
  ;[1 1 1] Begin play event
  (bind _returnvalue (Utilities|GetDataTableRow "/Game/Blueprint/Stats_DataTable.Stats_DataTable" "ShurikenBaseLifeSpan")
    (:then
      (Actor|SetLifeSpan (.value _returnvalue))
      (Utilities|FlowControl|Delay 0.0)
      (CallFunction|OnBeginPlay)
      ;[1 1 1] To give time to set things on the beginplay
      (Collision|BindEventtoOnActorHit (delegate Custom|Hit))
      (Collision|BindEventtoOnComponentBeginOverlap (Variables|Default|GetProjectileMesh) (delegate Custom|Overlapped))
      (Components|Activation|Activate (Variables|Default|GetProjectileMovement) false)
      (Collision|SetCollisionEnabled (Variables|Default|GetProjectileMesh) "QueryAndPhysics"))))

(fn ConstructionScript
  (Utilities|SetSpeedandScale)
  (Default|RicochetonConstruction (Variables|Default|GetBPC_Shuriken_Ricochet))
  (Default|ExplosiononConstruction (Variables|Default|GetBPC_Shuriken_Explosion)))

(fn DestroyLogic
  (params (Hit :type Boolean))
  (bind _effects (Variables|Default|GetEffects))
  (bind _effects_2 (Variables|Default|GetEffects))
  (bind _returnvalue (Utilities|Array|ContainsItem _effects "NewEnumerator3"))
  (bind _returnvalue_2 (Utilities|Array|ContainsItem _effects_2 "NewEnumerator4"))
  (bind _returnvalue_3 (or _returnvalue_2 _returnvalue))
  (bind _returnvalue_4 (select _returnvalue_3 0.6 1.0))
  (if (or Hit (not (Utilities|Array|ContainsItem (Variables|Default|GetEffects) "NewEnumerator2")))
    (if (and (Utilities|IsValid (Variables|Default|GetProjectileMesh)) (Utilities|IsValid (Variables|Default|GetAudioLife)))
      (if Hit
        (Audio|PlaySoundatLocation "/Game/Ultimate_SFX_Bundle/ultimate_Medieval_Combat_SFX/Bow_Arrow_Pro/Wavs/Arrow_Impact_Brick/Arrow_Impact_Brick_5.Arrow_Impact_Brick_5" (Transformation|GetWorldLocation (Variables|Default|GetProjectileMesh)) "0, 0, 0" 0.75 1.0 0.0 "/Game/Ultimate_SFX_Bundle/ShurikenSound_AttenuationSettings.ShurikenSound_AttenuationSettings" 0 0)
        (else
          (Audio|PlaySoundatLocation "/Game/Ultimate_SFX_Bundle/ultimate_Medieval_Combat_SFX/Bow_Arrow_Pro/Wavs/Arrow_Impact_wood/Arrow_Impact_wood_1_HighPitch.Arrow_Impact_wood_1_HighPitch" (Transformation|GetWorldLocation (Variables|Default|GetProjectileMesh)) "0, 0, 0" _returnvalue_4 1.0 0.0 "/Game/Ultimate_SFX_Bundle/ShurikenSound_AttenuationSettings.ShurikenSound_AttenuationSettings" 0 0)))
      (Audio|Components|Audio|Stop (Variables|Default|GetAudioLife)))
    (Actor|DestroyActor)
    (else
      (Audio|PlaySoundatLocation "/Game/Ultimate_SFX_Bundle/ultimate_Medieval_Combat_SFX/Bow_Arrow_Pro/Wavs/Arrow_Impact_wood/Arrow_Impact_wood_1_HighPitch.Arrow_Impact_wood_1_HighPitch" (Transformation|GetWorldLocation (Variables|Default|GetProjectileMesh)) "0, 0, 0" _returnvalue_4 1.0 0.0 "/Game/Ultimate_SFX_Bundle/ShurikenSound_AttenuationSettings.ShurikenSound_AttenuationSettings" 0 0))))

(fn BeforeDestroyOntHit
  (params (OtherActor :type Actor%20Object%20Reference) (Hit :type Hit%20Result%20Structure))
  (if (Utilities|Array|ContainsItem (Variables|Default|GetEffects) "NewEnumerator5")
    (Default|ExplosionBeforeDestroy (Variables|Default|GetBPC_Shuriken_Explosion))))

(fn BeforeDestroyonEnemy
  (params (OtherActor :type Actor%20Object%20Reference))
  (bind _effects (Variables|Default|GetEffects))
  (Utilities|IsValid OtherActor
    (:Is%20Valid
      (Utilities|FlowControl|Sequence
        (:then_0
          ;[1 1 1] Stun
          (if (Utilities|Array|ContainsItem (Variables|Default|GetEffects) "NewEnumerator1")
            (Default|StunBeforeDestroyEnemy (Variables|Default|GetBPC_Shuriken_Stun) OtherActor)))
        (:then_1
          ;[1 1 1] Ricochet
          (if (Utilities|Array|ContainsItem _effects "NewEnumerator3")
            (Default|RicochetBeforeDestroyEnemy (Variables|Default|GetBPC_Shuriken_Ricochet) OtherActor _effects)))
        (:then_2
          ;[1 1 1] Poison
          (if (Utilities|Array|ContainsItem (Variables|Default|GetEffects) "NewEnumerator6")
            (Default|PoisonBeforeDestroyEnemy (Variables|Default|GetBPC_Shuriken_Poison) OtherActor)))
        (:then_3
          ;[1 1 1] Explosion
          (if (Utilities|Array|ContainsItem (Variables|Default|GetEffects) "NewEnumerator5")
            (Default|ExplosionBeforeDestroy (Variables|Default|GetBPC_Shuriken_Explosion))))
        (:then_4
          ;[1 1 1] Dmg input
          (bind _returnvalue (Utilities|GetDataTableRow "/Game/Blueprint/Stats_DataTable.Stats_DataTable" "ShurikenBaseDamage")
            (:then
              (Utilities|IsValid OtherActor
                (:Is%20Valid
                  (Class|BPIDamage|DmgInput(Message) OtherActor (Math|Float|SelectFloat (* (.value _returnvalue) 2.0) (.value _returnvalue) (Utilities|Array|ContainsItem (Variables|Default|GetEffects) "NewEnumerator7")) "NewEnumerator0"))))))))))

(fn OnBeginPlay
  (Utilities|FlowControl|Sequence
    (:then_0
      ;[1 1 1] Big Effect
      (if (Utilities|Array|ContainsItem (Variables|Default|GetEffects) "NewEnumerator7")
        (Default|BigonBeginPlay (Variables|Default|GetBPC_Shuriken_Big))))
    (:then_1
      ;[1 1 1] Multiple
      (if (Utilities|Array|ContainsItem (Variables|Default|GetEffects) "NewEnumerator4")
        (Default|MultipleonBeginPlay (Variables|Default|GetBPC_Shuriken_Multiple) (Variables|Default|GetEffects))))
    (:then_2
      (return))))

(fn DmgInput
  (params (Damages :type Float%20%28single-precision%29) (AttackType :type EShurikenEffects%20Enum :default "NewEnumerator0"))
  (return))