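; BP_IntroPawn is an intro pawn that shows the main menu over a slowly rotating camera.
; On BeginPlay it creates the UI_MainMenu widget for the first player, adds it to the viewport, then moves CameraRoot to the world origin with a random starting yaw.
; Tick adds a small delta-time-scaled yaw to CameraRoot, giving a steady, frame-rate-independent orbit.
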(event EventBeginPlay
  (bind _returnvalue (UserInterface|CreateWidget "/Game/UI/UI_MainMenu.UI_MainMenu_C" (Game|GetPlayerController 0)))
  (bind _output_get (Variables|Default|SetUI _returnvalue))
  (UserInterface|Viewport|AddtoViewport _output_get 0)
  ;[1 1 1] For camera rotation
  (Transformation|SetWorldLocation (Variables|Default|GetCameraRoot) "0, 0, 0" false false)
  (Transformation|SetWorldRotation (Variables|Default|GetCameraRoot) (Math|Rotator|MakeRotator 0.0 0.0 (Math|Random|RandomFloatinRange -179.0 179.0)) false false))

(event EventTick
  (params (DeltaSeconds :type Float%20%28single-precision%29))
  ;[1 1 1] Camera rotation
  (Transformation|AddWorldRotation (Variables|Default|GetCameraRoot) (Math|Rotator|MakeRotator 0.0 0.0 (* (Utilities|Time|GetWorldDeltaSeconds) 2.5)) false false))

(fn ConstructionScript)