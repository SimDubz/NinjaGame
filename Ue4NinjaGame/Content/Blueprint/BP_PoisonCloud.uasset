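; BP_PoisonCloud is a poison zone, tied to shuriken stats, that damages enemies inside it over time.
; The construction script reads radius and duration from a stats data table, sizing the sphere, scaling Niagara thickness and density to match, and setting lifespan.
; On BeginPlay, a self-repeating event damages overlapping BP_BaseEnemy actors at a table-driven tick interval.
; Niagara density drops to zero after a short delay, while damage ticks continue.
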(event Custom|DealPoisonDmg
  (bind _returnvalue (Utilities|GetDataTableRow "/Game/Blueprint/Stats_DataTable.Stats_DataTable" "ShurikenPoisonDamage")
    (:then
      (Class|BPIDamage|DmgInput(Message) (Collision|GetOverlappingActors (Variables|Default|GetSphere) "/Game/Blueprint/BP_BaseEnemy.BP_BaseEnemy_C" :!class /Script/Engine.PrimitiveComponent) (.value _returnvalue) "NewEnumerator6")
      (bind _returnvalue_2 (Utilities|GetDataTableRow "/Game/Blueprint/Stats_DataTable.Stats_DataTable" "ShurikenPoisonTickTime")
        (:then
          (Utilities|FlowControl|Delay (.value _returnvalue_2))
          (CallFunction|DealPoisonDmg))))))

(event EventBeginPlay
  (CallFunction|DealPoisonDmg)
  (Utilities|FlowControl|Delay 1.0)
  (Effects|Components|ParticleSystem|SetFloatParameter (Variables|Default|GetNiagara) "Density" 0.0))

(fn ConstructionScript
  (bind _sphere (Variables|Default|GetSphere))
  (bind _niagara (Variables|Default|GetNiagara))
  (bind _returnvalue (Components|Sphere|GetScaledSphereRadius _sphere))
  (bind _returnvalue_2 (/ _returnvalue 75.0))
  (bind _returnvalue_3 (Utilities|GetDataTableRow "/Game/Blueprint/Stats_DataTable.Stats_DataTable" "ShurikenPoisionZoneRadius")
    (:then
      (Components|Sphere|SetSphereRadius (Variables|Default|GetSphere) (.value _returnvalue_3) true)
      (Effects|Components|ParticleSystem|SetFloatParameter _niagara "Thickness" (* _returnvalue_2 1.0))
      (Effects|Components|ParticleSystem|SetFloatParameter _niagara "Density" (* _returnvalue_2 5e+01))
      (bind _returnvalue_4 (Utilities|GetDataTableRow "/Game/Blueprint/Stats_DataTable.Stats_DataTable" "ShurikenPoisonDuration")
        (:then
          (Actor|SetLifeSpan (.value _returnvalue_4)))))))