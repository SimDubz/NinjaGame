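; BP_BossProjectile is a boss projectile that plays a fire bolt sound when it spawns.
; Its sphere overlap responds only to BP_BasePawn actors, calling DmgInput on them with damage set to zero.
; It then plays an explosion sound at its own location, spawns an energy explosion effect at the pawn's location and destroys itself.
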(event OnComponentBeginOverlap(Sphere)
  (params (OverlappedComponent :type Primitive%20Component%20Object%20Reference) (OtherActor :type Actor%20Object%20Reference) (OtherComp :type Primitive%20Component%20Object%20Reference) (OtherBodyIndex :type Integer) (bFromSweep :type Boolean) (SweepResult :type Hit%20Result%20Structure%20%28by%20ref%29))
  (bind _asbp_base_pawn (Utilities|Casting|CastToBP_BasePawn OtherActor))
  (Default|DmgInput _asbp_base_pawn 0.0 "NewEnumerator0")
  (Audio|PlaySoundatLocation "/Game/Ultimate_SFX_Bundle/Explosion_Sounds_Pro/Wavs/Explosion_Tiny_04.Explosion_Tiny_04" (Transformation|GetWorldLocation (Variables|Default|GetDefaultSceneRoot)) "0, 0, 0" 1.0 1.0 0.0 0 0 0)
  (Niagara|SpawnSystematLocation "/Game/Marketplace/Stylized_VFX_StPack/P_ExplosionEnergy_02.P_ExplosionEnergy_02" (Transformation|GetActorLocation _asbp_base_pawn))
  (Actor|DestroyActor))

(event EventBeginPlay
  (Audio|PlaySoundatLocation "/Game/Ultimate_SFX_Bundle/ultimate_Medieval_Combat_SFX/Magic_SFX_Pro/Wavs/Fire_Bolts/Fire_bolt_4.Fire_bolt_4" (Transformation|GetWorldLocation (Variables|Default|GetDefaultSceneRoot)) "0, 0, 0" 1.0 1.0 0.0 0 0 0) ; Projectile spawn
)

(fn ConstructionScript)