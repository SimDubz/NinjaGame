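; Third-person player character with axis-driven movement, jump, turn-rate-scaled camera look and pitch limits set on BeginPlay.
; Overrides RotateToCursor as a no-op, suggesting a parent built for cursor aiming.
; Dash teleports along flattened input direction, or forward when idle, stopping at WorldStatic hits, though its distance multiplier is zero.
; Shuriken spawning traces from the camera, aiming the socket-spawned projectile at the hit point, otherwise along camera rotation.
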(event EventBeginPlay
  (bind _returnvalue (Game|GetPlayerCameraManager 0))
  (|CallParentFunction)
  (Pawn|SetControlRotation (Pawn|GetController) (Transformation|GetWorldRotation (Variables|Default|GetSpringArm)))
  (Variables|/Script/Engine.PlayerCameraManager|SetViewPitchMax _returnvalue 25.0)
  (Variables|/Script/Engine.PlayerCameraManager|SetViewPitchMin _returnvalue -6e+01))

(event Collision|EventActorBeginOverlap
  (params (OtherActor :type Actor%20Object%20Reference)))

(event EventTick
  (params (DeltaSeconds :type Float%20%28single-precision%29))
  (|CallParentFunction DeltaSeconds) ; This node is disabled and will not be called.\nDrag off pins to build functionality.
)

(event Input|ActionEvents|InputActionJump
  (params (Key :type Key%20Structure))
  (:Pressed
    (Character|Jump)))

(event Input|AxisEvents|InputAxisForward
  (params (AxisValue :type Float%20%28single-precision%29))
  (Pawn|Input|AddMovementInput (Math|Vector|GetForwardVector (Variables|Default|GetCapsuleComponent)) AxisValue false))

(event Input|AxisEvents|InputAxisPitchInput
  (params (AxisValue :type Float%20%28single-precision%29))
  (Pawn|Input|AddControllerPitchInput (* (* AxisValue (Variables|Default|GetBaseTurnRate) (Utilities|Time|GetWorldDeltaSeconds)) -1.0)))

(event Input|AxisEvents|InputAxisRight
  (params (AxisValue :type Float%20%28single-precision%29))
  (Pawn|Input|AddMovementInput (Math|Vector|GetRightVector (Variables|Default|GetCapsuleComponent)) AxisValue false))

(event Input|AxisEvents|InputAxisYawInput
  (params (AxisValue :type Float%20%28single-precision%29))
  (Pawn|Input|AddControllerYawInput (* AxisValue (Variables|Default|GetBaseTurnRate) (Utilities|Time|GetWorldDeltaSeconds))))

(fn ConstructionScript
  (|CallParentFunction))

(fn RotatetoCursor)

(fn Dash
  (bind _returnvalue (Input|AxisValues|GetForward))
  (bind _returnvalue_2 (Input|AxisValues|GetRight))
  (bind _capsulecomponent (Variables|Default|GetCapsuleComponent))
  (bind _capsulecomponent_2 (Variables|Default|GetCapsuleComponent))
  (bind _capsulecomponent_3 (Variables|Default|GetCapsuleComponent))
  (bind _returnvalue_3 (== _returnvalue 0.0))
  (bind _returnvalue_4 (== _returnvalue_2 0.0))
  (bind _returnvalue_5 (Math|Vector|GetForwardVector _capsulecomponent_3))
  (bind _returnvalue_6 (Math|Vector|GetForwardVector _capsulecomponent))
  (bind _returnvalue_7 (Math|Vector|GetRightVector _capsulecomponent))
  (bind _returnvalue_8 (Transformation|GetWorldLocation _capsulecomponent_2))
  (bind _returnvalue_9 (* _returnvalue_6 _returnvalue))
  (bind _returnvalue_10 (* _returnvalue_7 _returnvalue_2))
  (bind _returnvalue_11 (and _returnvalue_3 _returnvalue_4))
  (bind _returnvalue_12 (+ _returnvalue_9 _returnvalue_10))
  (bind _returnvalue_13 (select _returnvalue_11 _returnvalue_5 _returnvalue_12))
  (bind (_x _y) (Math|Vector|BreakVector _returnvalue_13))
  (bind _returnvalue_14 (* (Math|Vector|MakeVector _x _y 0.0) 0.0))
  (bind _returnvalue_15 (+ _returnvalue_8 _returnvalue_14))
  (bind (_outhit _returnvalue_16) (Collision|LineTraceForObjects _returnvalue_8 _returnvalue_15 (Utilities|Array|MakeArray "ObjectTypeQuery1") false 0 "None"))
  (Transformation|Teleport (select _returnvalue_16 (.Location (Collision|BreakHitResult _outhit)) _returnvalue_15) (Transformation|GetWorldRotation (Variables|Default|GetCapsuleComponent)))
  (return))

(fn SpawnShurikenProjectile
  (bind _camera (Variables|Default|GetCamera))
  (bind _returnvalue (Transformation|GetWorldLocation _camera))
  ;[1 1 1] Spawn Projectile at location
  (bind (_outhit _returnvalue_2) (Collision|LineTraceByChannel _returnvalue (+ _returnvalue (* (Math|Vector|GetForwardVector _camera) 1e+04)) "TraceTypeQuery1" true 0 "None"))
  (bind _returnvalue_3 (Game|SpawnActorfromClass "/Game/Blueprint/BP_Shuriken.BP_Shuriken_C" (Math|Transform|MakeTransform (.location (Transformation|GetSocketTransform (Variables|Character|GetMesh) "Socket_Shuriken" "RTS_World")) (select _returnvalue_2 (Math|Rotator|FindLookatRotation (.location (Transformation|GetSocketTransform (Variables|Character|GetMesh) "Socket_Shuriken" "RTS_World")) (.Location (Collision|BreakHitResult _outhit))) (Camera|GetCameraRotation (Variables|/Script/Engine.PlayerController|GetPlayerCameraManager (Game|GetPlayerController 0)))) "1.500000,1.500000,1.500000") "AlwaysSpawn" 0 0))
  (Utilities|IsValid _returnvalue_3
    (:Is%20Valid
      (Actor|SetLifeSpan _returnvalue_3 4.0))))