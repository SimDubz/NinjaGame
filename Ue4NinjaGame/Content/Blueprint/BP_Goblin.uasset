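; Goblin character that wanders random navigable points within the BP_BaseSpawner's BlockSphere and drops a random ability pickup when killed.
; Construction script reads lifespan, walk speed and health from a stats data table; AIMoveTo re-triggers itself on success or failure.
; DmgInput lowers health, drives a crack material parameter from the health ratio, and plays hit effects or handles death.
; Any destruction, including lifespan expiry, spawns an emitter via OnDestroyed.
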(event Custom|WalkToRandomDest
  (bind _spawnsphere (Variables|Default|GetSpawnSphere))
  ;[1 1 1] Walk to random destination
  (bind _randomlocation (Class|NavigationSystemV1|GetRandomLocationinNavigableRadius (Transformation|GetWorldLocation _spawnsphere) (Variables|/Script/Engine.SphereComponent|GetSphereRadius _spawnsphere) 0 0))
  (AI|AIMoveTo self _randomlocation 0 5.0 false
    (:OnSuccess
      _)
    (:OnFail
      _))
  (CallFunction|WalktoRandomDest))

(event Custom|Destroy%20Emitter
  (params (DestroyedActor :type Actor%20Object%20Reference))
  ;[1 1 1] On destroy emitter
  (Effects|SpawnEmitteratLocation "/Game/Marketplace/AdvancedMagicFX12/particles/P_ky_hit.P_ky_hit" (Transformation|GetWorldLocation (Variables|Collision|GetCapsuleComponent))))

(event EventBeginPlay
  ;[1 1 1] Begin Play
  (bind _returnvalue (Actor|GetActorOfClass "/Game/Blueprint/BP_BaseSpawner.BP_BaseSpawner_C"))
  (Utilities|IsValid _returnvalue
    (:Is%20Valid
      (Variables|Default|SetSpawnSphere (Variables|/Game/Blueprint/BP_BaseSpawner.BP_BaseSpawner_C|GetBlockSphere _returnvalue))
      (CallFunction|WalktoRandomDest)
      ;[1 1 1] On destroy emitter
      (Game|AssignOnDestroyed (delegate Custom|Destroy%20Emitter)))))

(event EventDmgInput
  (params (Damages :type Float%20%28single-precision%29) (AttackType :type EShurikenEffects%20Enum :default "NewEnumerator0"))
  (bind _capsulecomponent (Variables|Collision|GetCapsuleComponent))
  (bind _capsulecomponent_2 (Variables|Collision|GetCapsuleComponent))
  ;[1 1 1] On hit logic
  (if (not (Variables|Default|GetIsDead))
    (bind _output_get (Variables|Default|SetHealth (- (Variables|Default|GetHealth) Damages)))
    ;;[1 1 1] To update health visual
    (bind _returnvalue (Utilities|GetDataTableRow "/Game/Blueprint/Stats_DataTable.Stats_DataTable" "GolbinBaseHealth")
      (:then
        (Rendering|Material|SetScalarParameterValueonMaterials (Variables|Default|GetStaticMesh) "CracksIntensity" (/ (Variables|Default|GetHealth) (.value _returnvalue)))
        (if (<= _output_get 0.0)
          (Variables|Default|SetIsDead true)
          ;[1 1 1] Before destroy if hitted
          (Game|SpawnActorfromClass "/Game/Blueprint/AltShurikens/BP_AbilityPickup_Random.BP_AbilityPickup_Random_C" (Math|Transform|MakeTransform (- (Transformation|GetWorldLocation _capsulecomponent_2) (Math|Vector|MakeVector 0.0 0.0 (Variables|/Script/Engine.CapsuleComponent|GetCapsuleHalfHeight _capsulecomponent_2))) "0, 0, 0" "1,1,1") "Undefined" 0 0)
          (Utilities|FlowControl|Delay 0.0) ; To have time to run code before
          (Actor|DestroyActor)
          (else
            ;[1 1 1] Hit particle
            (Niagara|SpawnSystemAttached "/Game/Marketplace/Stylized_VFX_StPack/Particles/UPDATE_1_3/P_Web_Hit_01.P_Web_Hit_01" _capsulecomponent "" (Math|Vector|MakeVector (Variables|/Script/Engine.CapsuleComponent|GetCapsuleRadius _capsulecomponent) 0.0 0.0) "0, 0, 0" "SnapToTargetIncludingScale" true)))))))

(fn ConstructionScript
  (bind _returnvalue (Utilities|GetDataTableRow "/Game/Blueprint/Stats_DataTable.Stats_DataTable" "GolbinBaseDuration")
    (:then
      (Actor|SetLifeSpan self (.value _returnvalue))
      (bind _returnvalue_2 (Utilities|GetDataTableRow "/Game/Blueprint/Stats_DataTable.Stats_DataTable" "GolbinBaseSpeed")
        (:then
          (Variables|/Script/Engine.CharacterMovementComponent|SetMaxWalkSpeed (Variables|Character|GetCharacterMovement) (.value _returnvalue_2))
          (bind _returnvalue_3 (Utilities|GetDataTableRow "/Game/Blueprint/Stats_DataTable.Stats_DataTable" "GolbinBaseHealth")
            (:then
              (Variables|Default|SetHealth (.value _returnvalue_3)))))))))