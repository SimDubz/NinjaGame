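; Heart pickup that raises the health of a BP_BasePawn that touches it.
; Sphere overlap casts the other actor to BP_BasePawn and calls IncreaseHealth; when that returns false, the pickup plays a power-up sound and destroys itself.
; The construction script sets the actor's lifespan from the PickupDuration row of a stats data table, so uncollected hearts expire.
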(event OnComponentBeginOverlap(Sphere)
  (params (OverlappedComponent :type Primitive%20Component%20Object%20Reference) (OtherActor :type Actor%20Object%20Reference) (OtherComp :type Primitive%20Component%20Object%20Reference) (OtherBodyIndex :type Integer) (bFromSweep :type Boolean) (SweepResult :type Hit%20Result%20Structure%20%28by%20ref%29))
  (CallFunction|GiveHearttoPlayer OtherActor))

(fn ConstructionScript
  (bind _returnvalue (Utilities|GetDataTableRow "/Game/Blueprint/Stats_DataTable.Stats_DataTable" "PickupDuration")
    (:then
      (Actor|SetLifeSpan (.value _returnvalue)))))

(fn GiveHearttoPlayer
  (params (PlayerActor :type Object%20Object%20Reference))
  (bind _asbp_base_pawn (Utilities|Casting|CastToBP_BasePawn PlayerActor))
  (bind _alreadyfull (Default|IncreaseHealth _asbp_base_pawn))
  (if (not _alreadyfull)
    (Audio|PlaySoundatLocation "/Game/Ultimate_SFX_Bundle/Modern_Ui_Sounds/Wavs/Power_Up_Sounds/Power_Up_Sound_1.Power_Up_Sound_1" (Transformation|GetWorldLocation (Variables|Default|GetDefaultSceneRoot)) "0, 0, 0" 1.0 1.0 0.0 0 0 0)
    (Actor|DestroyActor)))