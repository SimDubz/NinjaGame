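; Shuriken component for the Big variant that enlarges its owning shuriken through the BigOnBeginPlay function.
; It multiplies the owner's actor scale by a factor read from the stats data table.
; On a BP_Shuriken owner, it also sets the relative scale of the ricochet and explosion range spheres to that factor times a table-driven ratio, only when the product is at least one.
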(fn BigonBeginPlay
  (bind _returnvalue (Components|GetOwner))
  (Utilities|IsValid _returnvalue
    (:Is%20Valid
      (bind _returnvalue_2 (Utilities|GetDataTableRow "/Game/Blueprint/Stats_DataTable.Stats_DataTable" "ShurikenBigScale")
        (:then
          (Transformation|SetActorScale3D _returnvalue (* (Transformation|GetActorScale3D _returnvalue) (.value _returnvalue_2)))
          (bind _asbp_shuriken (Utilities|Casting|CastToBP_Shuriken (Components|GetOwner)))
          ;[1 1 1] Set scale on sphere radius
          (bind _returnvalue_3 (Utilities|GetDataTableRow "/Game/Blueprint/Stats_DataTable.Stats_DataTable" "ShurikenBigScaleRatio")
            (:then
              (if (>= (* (.value _returnvalue_2) (.value _returnvalue_3)) 1.0)
                (Transformation|SetRelativeScale3D (Variables|/Game/Blueprint/BP_Shuriken.BP_Shuriken_C|GetRangeSphere_Ricochet _asbp_shuriken) (* "1.000000,1.000000,1.000000" (* (.value _returnvalue_2) (.value _returnvalue_3))))))))))))