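; Shuriken component variant that fires a fan of additional BP_Shuriken projectiles from the player pawn on BeginPlay.
; It reads count and spread angle from a stats data table, spawning from the second shuriken onward at yaw offsets alternating either side, widening after each pair.
; ShurikenSpawn places each at the pawn's Socket_Shuriken relative to actor rotation, adds the base shuriken component and sets lifespan from the table.
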(event EventBeginPlay
  (|CallParentFunction)
  (bind _returnvalue (Utilities|GetDataTableRow "/Game/Blueprint/Stats_DataTable.Stats_DataTable" "ShurikenMultipleCounter")
    (:then
      (for _index (range 2 (Math|Float|Truncate (.value _returnvalue)))
        (bind _returnvalue_2 (Utilities|GetDataTableRow "/Game/Blueprint/Stats_DataTable.Stats_DataTable" "ShurikenMultipleAngle")
          (:then
            (Utilities|FlowControl|FlipFlop
              (:A
                (CallFunction|ShurikenSpawn (Math|Rotator|MakeRotator 0.0 0.0 (* (.value _returnvalue_2) (Variables|Default|GetDegreeMultiplier)))))
              (:B
                (CallFunction|ShurikenSpawn (Math|Rotator|MakeRotator 0.0 0.0 (* (* (.value _returnvalue_2) -1.0) (Variables|Default|GetDegreeMultiplier))))
                (Math|Float|IncrementFloat (Variables|Default|GetDegreeMultiplier))))))))))

(fn ShurikenSpawn
  (params (InputRotationOffset :type Rotator))
  (bind _returnvalue (Game|Player|GetPlayerPawn 0))
  ;[1 1 1] Spawn Projectile at location
  (bind _asbp_base_pawn (Utilities|Casting|CastToBP_BasePawn _returnvalue))
  (bind _returnvalue_2 (Game|SpawnActorfromClass "/Game/Blueprint/BP_Shuriken.BP_Shuriken_C" (Math|Transform|MakeTransform (.location (Transformation|GetSocketTransform (Variables|/Script/Engine.Character|GetMesh _asbp_base_pawn) "Socket_Shuriken" "RTS_World")) (Math|Rotator|CombineRotators InputRotationOffset (Transformation|GetActorRotation _returnvalue))) "AlwaysSpawn" 0 0))
  ;[1 1 1] Set Shuriken Components
  (Utilities|IsValid _returnvalue_2
    (:Is%20Valid
      (Game|AddComponentbyClass _returnvalue_2 "/Game/Blueprint/AltShurikens/BPC_Shuriken_Base.BPC_Shuriken_Base_C")
      (bind _returnvalue_3 (Utilities|GetDataTableRow "/Game/Blueprint/Stats_DataTable.Stats_DataTable" "ShurikenBaseLifeSpan")
        (:then
          (Actor|SetLifeSpan _returnvalue_2 (.value _returnvalue_3)))))))