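; BP_AbilityPickup is a world pickup that grants a shuriken effect to a pawn that touches it.
; A sphere overlap calls GiveAbilityToPlayer, which accepts only BP_BasePawn actors, plays a buff sound, adds the configured ShurikenEffect to the pawn and destroys itself.
; The construction script tints the cube's materials with ObjectColor through a vector parameter.
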(event OnComponentBeginOverlap(Sphere)
  (params (OverlappedComponent :type Primitive%20Component%20Object%20Reference) (OtherActor :type Actor%20Object%20Reference) (OtherComp :type Primitive%20Component%20Object%20Reference) (OtherBodyIndex :type Integer) (bFromSweep :type Boolean) (SweepResult :type Hit%20Result%20Structure%20%28by%20ref%29))
  (CallFunction|GiveAbilitytoPlayer OtherActor))

(fn ConstructionScript
  (Rendering|Material|SetVectorParameterValueonMaterials (Variables|Default|GetCube) "Color" (Math|Conversions|ToVector(LinearColor) (Variables|Default|GetObjectColor))))

(fn GiveAbilitytoPlayer
  (params (PlayerActor :type Object%20Object%20Reference))
  (bind _asbp_base_pawn (Utilities|Casting|CastToBP_BasePawn PlayerActor))
  (Audio|PlaySoundatLocation "/Game/Ultimate_SFX_Bundle/ultimate_Medieval_Combat_SFX/Magic_SFX_Pro/Wavs/Buffs/Buff_18.Buff_18" (Transformation|GetWorldLocation (Variables|Default|GetDefaultSceneRoot)) "0, 0, 0" 1.0 1.0 0.0 0 0 0)
  (Default|AddShurikenEffect _asbp_base_pawn (Variables|Default|GetShurikenEffect))
  (Actor|DestroyActor))