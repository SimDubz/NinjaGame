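; Shuriken component for the poison variant that spawns a poison cloud through its before-destroy-enemy function.
; The cloud appears at the owning shuriken's X/Y location at a fixed height.
; Its scale comes from stats data table rows: big scale times its ratio when the shuriken has a particular effect, otherwise the shuriken's scale divided by base size.
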(fn PoisonBeforeDestroyEnemy
  (params (Actor :type Actor%20Object%20Reference))
  (bind _returnvalue (Components|GetOwner))
  (bind _returnvalue_2 (Transformation|GetActorLocation _returnvalue))
  (bind _asbp_shuriken (Utilities|Casting|CastToBP_Shuriken _returnvalue))
  (bind _returnvalue_3 (Utilities|GetDataTableRow "/Game/Blueprint/Stats_DataTable.Stats_DataTable" "ShurikenBaseSize")
    (:then
      (bind _returnvalue_4 (Utilities|GetDataTableRow "/Game/Blueprint/Stats_DataTable.Stats_DataTable" "ShurikenBigScale")
        (:then
          (bind _returnvalue_5 (Utilities|GetDataTableRow "/Game/Blueprint/Stats_DataTable.Stats_DataTable" "ShurikenBigScaleRatio")
            (:then
              (Game|SpawnActorfromClass "/Game/Blueprint/BP_PoisonCloud.BP_PoisonCloud_C" (Math|Transform|MakeTransform (Math|Vector|MakeVector (.x _returnvalue_2) (.y _returnvalue_2) 1e+02) "0, 0, 0" (Math|Vector|SelectVector (Math|Conversions|ToVector(Float) (* (.value _returnvalue_4) (.value _returnvalue_5))) (/ (Transformation|GetActorScale3D _returnvalue) (.value _returnvalue_3)) (Utilities|Array|ContainsItem (Variables|/Game/Blueprint/BP_Shuriken.BP_Shuriken_C|GetEffects _asbp_shuriken) "NewEnumerator7"))) "Undefined" 0 0))))))))