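; Actor component for BP_Shuriken that adds an area explosion dealing damage to nearby enemies before the shuriken is destroyed.
; On construction it sizes the owner's RangeSphereExplosion from the explosion range row in the stats DataTable.
; Before destroy it spawns a fire hit particle scaled to the sphere radius, then sends table-driven damage to every overlapping BP_BaseEnemy through DmgInputMessage.
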(fn ExplosionBeforeDestroy
  (bind _returnvalue (Components|GetOwner))
  (bind _asbp_shuriken (Utilities|Casting|CastToBP_Shuriken _returnvalue))
  (Effects|SpawnEmitteratLocation "/Game/Marketplace/AdvancedMagicFX12/particles/P_ky_hit_fire.P_ky_hit_fire" (Transformation|GetActorLocation _returnvalue) "0, 0, 0" (* "1.000000,1.000000,1.000000" (/ (Components|Sphere|GetScaledSphereRadius (Variables|/Game/Blueprint/BP_Shuriken.BP_Shuriken_C|GetRangeSphere_Explosion _asbp_shuriken)) 175.0)))
  (bind _output_get (LocalVariables|SetOverlappingACtors (Collision|GetOverlappingActors (Variables|/Game/Blueprint/BP_Shuriken.BP_Shuriken_C|GetRangeSphere_Explosion _asbp_shuriken) "/Game/Blueprint/BP_BaseEnemy.BP_BaseEnemy_C" :!class /Script/Engine.PrimitiveComponent)))
  (for _array_element _output_get
    (Utilities|IsValid _array_element
      (:Is%20Valid
        (bind _returnvalue_2 (Utilities|GetDataTableRow "/Game/Blueprint/Stats_DataTable.Stats_DataTable" "ShurikenExplosionDamage")
          (:then
            (Class|BPIDamage|DmgInput(Message) _array_element (.value _returnvalue_2) "NewEnumerator0")))))))

(fn ExplosiononConstruction
  (bind _asbp_shuriken (Utilities|Casting|CastToBP_Shuriken (Components|GetOwner)))
  (bind _returnvalue (Utilities|GetDataTableRow "/Game/Blueprint/Stats_DataTable.Stats_DataTable" "ShurikenExplosionRange")
    (:then
      (Components|Sphere|SetSphereRadius (Variables|/Game/Blueprint/BP_Shuriken.BP_Shuriken_C|GetRangeSphere_Explosion _asbp_shuriken) (.value _returnvalue) true))))