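; Player ninja pawn for top-down combat, with axis movement, cursor-facing rotation, melee slice, shuriken throw and dash.
; Montage notifies toggle the melee hitbox, which damages each enemy once per swing, while a separate Throw event spawns short-lived shurikens from a hand socket.
; Dash teleports along input or facing, stopped by world-static traces.
; UI_Base shows health, score and time; death shows game over, disables input and closes the Tick gate.
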(event OnComponentBeginOverlap(MeleeBox)
  (params (OverlappedComponent :type Primitive%20Component%20Object%20Reference) (OtherActor :type Actor%20Object%20Reference) (OtherComp :type Primitive%20Component%20Object%20Reference) (OtherBodyIndex :type Integer) (bFromSweep :type Boolean) (SweepResult :type Hit%20Result%20Structure%20%28by%20ref%29))
  ;[1 0.3473 0.2776] Melee attack
  ;;[1 1 1] On hit logic
  (Utilities|MeleeHitLogic OtherActor))

(event Custom|StopTick
  ;[1 1 1] Look at cursor
  (Utilities|FlowControl|Gate false) ; enters at Close
)

(event Custom|Throw
  ;[1 0.8781 0.2304] Throw Shuriken
  ;;[1 1 1] SpawnShuriken
  (CallFunction|SpawnShurikenProjectile))

(event EventBeginPlay
  ;[1 1 1] Begin paly create UI
  (bind _returnvalue (UserInterface|CreateWidget "/Game/UI/UI_Base.UI_Base_C"))
  (bind _output_get (Variables|Default|SetWidget _returnvalue))
  (UserInterface|Viewport|AddtoViewport _output_get 0)
  (Variables|Default|SetHealth (Variables|Stats|GetInitialHealth)))

(event EventTick
  (params (DeltaSeconds :type Float%20%28single-precision%29))
  ;[1 1 1] Look at cursor
  (Utilities|FlowControl|Gate false
    (:Exit
      (Utilities|FlowControl|Sequence
        (:then_0
          (CallFunction|RotatetoCursor))
        (:then_1
          (Utilities|UpdateTimer))))))

(event EventDmgInput
  (params (Damages :type Float%20%28single-precision%29) (AttackType :type String))
  ;[1 1 1] Receive dmg logic
  (bind _isdead (Utilities|UpdateHealth Damages))
  (if _isdead
    (CallFunction|Die)))

(event Input|ActionEvents|InputActionDash
  (params (Key :type Key%20Structure :default "None"))
  ;[1 1 1] Dash
  (:Pressed
    (CallFunction|Dash)))

(event Input|ActionEvents|InputActionPrimary
  (params (Key :type Key%20Structure :default "None"))
  ;[1 0.3473 0.2776] Melee attack
  (:Pressed
    (if (not (Variables|Default|GetInAttack))
      (Variables|Default|SetInAttack true)
      (Utilities|Array|Clear (Variables|Default|GetHittedActor))
      (Animation|Montage|PlayMontage (Variables|Character|GetMesh) "/Game/Ninja/Animation/Anim_Ninja_Slice_01_Montage.Anim_Ninja_Slice_01_Montage" 1.5
        (:OnNotifyBegin
          (Collision|SetCollisionEnabled (Variables|Default|GetMeleeBox) "QueryOnly"))
        (:OnNotifyEnd
          (Variables|Default|SetInAttack false)
          (Collision|SetCollisionEnabled (Variables|Default|GetMeleeBox) "NoCollision"))))))

(event Input|ActionEvents|InputActionSecondary
  (params (Key :type Key%20Structure :default "None"))
  ;[1 0.8781 0.2304] Throw Shuriken
  (:Pressed
    (if (not (Variables|Default|GetInAttack))
      (Utilities|Array|Clear (Variables|Default|GetHittedActor))
      (Variables|Default|SetInAttack true)
      (Animation|Montage|PlayMontage (Variables|Character|GetMesh) "/Game/Ninja/Animation/Anim_Ninja_ShurikenThrow_Montage.Anim_Ninja_ShurikenThrow_Montage" 2.0
        (:OnCompleted
          (Variables|Default|SetInAttack false))))))

(event Input|AxisEvents|InputAxisForward
  (params (AxisValue :type Float%20%28single-precision%29))
  ;[1 1 1] Player Movement
  (Pawn|Input|AddMovementInput "1.000000,0.000000, 0" AxisValue false))

(event Input|AxisEvents|InputAxisRight
  (params (AxisValue :type Float%20%28single-precision%29))
  ;[1 1 1] Player Movement
  (Pawn|Input|AddMovementInput "0.000000,1.000000, 0" AxisValue false))

(fn ConstructionScript)

(fn RotatetoCursor
  (bind _returnvalue (Game|GetPlayerController 0))
  (bind _capsulecomponent (Variables|Collision|GetCapsuleComponent))
  (bind _hitresult (Game|Player|GetHitResultUnderCursorbyChannel _returnvalue "TraceTypeQuery1" true))
  (bind _returnvalue_2 (Transformation|GetWorldLocation _capsulecomponent))
  (bind _location (Collision|BreakHitResult _hitresult))
  (bind _returnvalue_3 (Math|Rotator|FindLookatRotation _returnvalue_2 _location))
  (Transformation|SetWorldRotation (Variables|Collision|GetCapsuleComponent) (Math|Rotator|MakeRotator 0.0 0.0 (.yaw _returnvalue_3)) false false)
  (Variables|Default|SetLookAtDirection (.yaw _returnvalue_3)))

(fn Die
  (Widget|SetVisibility (Variables|/Game/UI/UI_Base.UI_Base_C|GetGameOVer (Variables|Default|GetWidget)) "Visible")
  (Input|DisableInput (Game|GetPlayerController 0))
  (bind _asanim_bp_base (Utilities|Casting|CastToAnimBP_Base (Components|SkeletalMesh|GetAnimInstance (Variables|Character|GetMesh))))
  (Default|Death _asanim_bp_base)
  (CallFunction|StopTick))

(fn UpdateScore
  (params (points :type Integer))
  (bind _output_get (Variables|Default|SetScore (+ (Variables|Default|GetScore) points)))
  (Rendering|Components|TextRender|SetText (Variables|/Game/UI/UI_Base.UI_Base_C|GetScoreCounter (Variables|Default|GetWidget)) (Utilities|Text|ToText(Integer) _output_get))
  (return))

(fn Dash
  (bind _returnvalue (Input|AxisValues|GetForward))
  (bind _returnvalue_2 (Input|AxisValues|GetRight))
  (bind _dashdistance (Variables|Stats|GetDashDistance))
  (bind _capsulecomponent (Variables|Collision|GetCapsuleComponent))
  (bind _capsulecomponent_2 (Variables|Collision|GetCapsuleComponent))
  (bind _returnvalue_3 (== _returnvalue 0.0))
  (bind _returnvalue_4 (== _returnvalue_2 0.0))
  (bind _returnvalue_5 (Math|Vector|GetForwardVector _capsulecomponent_2))
  (bind _returnvalue_6 (Transformation|GetWorldLocation _capsulecomponent))
  (bind _returnvalue_7 (and _returnvalue_3 _returnvalue_4))
  (bind _returnvalue_8 (select _returnvalue_7 _returnvalue_5 (Math|Vector|MakeVector _returnvalue _returnvalue_2 0.0)))
  (bind (_x _y) (Math|Vector|BreakVector _returnvalue_8))
  (bind _returnvalue_9 (* (Math|Vector|MakeVector _x _y 0.0) _dashdistance))
  (bind _returnvalue_10 (+ _returnvalue_6 _returnvalue_9))
  (bind (_outhit _returnvalue_11) (Collision|LineTraceForObjects _returnvalue_6 _returnvalue_10 (Utilities|Array|MakeArray "ObjectTypeQuery1") false 0 "None"))
  (Transformation|Teleport (select _returnvalue_11 (.Location (Collision|BreakHitResult _outhit)) _returnvalue_10) (Transformation|GetWorldRotation (Variables|Collision|GetCapsuleComponent)))
  (return))

(fn SpawnShurikenProjectile
  ;[1 1 1] Spawn Projectile at location
  (bind _returnvalue (Game|SpawnActorfromClass "/Game/Blueprint/BP_Shuriken.BP_Shuriken_C" (Math|Transform|MakeTransform (.location (Transformation|GetSocketTransform (Variables|Character|GetMesh) "Socket_Shuriken" "RTS_World")) (Math|Conversions|RotationFromXVector (Math|Vector|GetForwardVector (Variables|Collision|GetCapsuleComponent))) "1.500000,1.500000,1.500000") "AlwaysSpawn" 0 0))
  (Utilities|IsValid _returnvalue
    (:Is%20Valid
      (Actor|SetLifeSpan _returnvalue 0.4))))