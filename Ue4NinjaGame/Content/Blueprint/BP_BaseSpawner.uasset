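; Spawner that continuously spawns base enemies, elites, bosses and goblins at random navmesh points around its SpawnSphere, retrying any point inside BlockSphere.
; Each type runs a self-recalling delay loop timed from Stats_DataTable; base enemies start immediately, the others after a delay.
; SpawnRateMath is meant to shorten all but goblin delays using a time-growing, capped divider, configured in the construction script.
; Sounds mark game start and boss spawns.
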(event Custom|SpawnUnit
  (bind _spawnsphere (Variables|Default|GetSpawnSphere))
  (bind _blocksphere (Variables|Default|GetBlockSphere))
  ;[1 1 1] SPawn normal units
  (bind _randomlocation (Class|NavigationSystemV1|GetRandomLocationinNavigableRadius (Transformation|GetWorldLocation _spawnsphere) (Components|Sphere|GetScaledSphereRadius _spawnsphere) 0 0))
  (if (> (Math|Vector|Distance(Vector) _randomlocation (Transformation|GetWorldLocation _blocksphere)) (Variables|/Script/Engine.SphereComponent|GetSphereRadius _blocksphere))
    (Game|SpawnActorfromClass "/Game/Blueprint/BP_BaseEnemy.BP_BaseEnemy_C" (Math|Transform|MakeTransform _randomlocation "0, 0, 0" "1,1,1") "Undefined" 0 0)
    (bind _returnvalue (Utilities|GetDataTableRow "/Game/Blueprint/Stats_DataTable.Stats_DataTable" "EnemyBaseSpawnRate")
      (:then
        (Utilities|FlowControl|Delay (Utilities|SpawnRateMath (.value _returnvalue))) ; Spawn Time
        (CallFunction|SpawnUnit)))
    (else
      (CallFunction|SpawnUnit))))

(event Custom|SpawnBoss
  (bind _spawnsphere (Variables|Default|GetSpawnSphere))
  (bind _blocksphere (Variables|Default|GetBlockSphere))
  ;[1 1 1] SPawn Boss units
  (Audio|PlaySoundatLocation "/Game/Ultimate_SFX_Bundle/Monster_Sounds_Pro/Wavs/Large_monster_laugh/Large_monster_laugh_2.Large_monster_laugh_2" "0, 0, 0" "0, 0, 0" 1.0 1.0 0.0 0 0 0)
  (bind _randomlocation (Class|NavigationSystemV1|GetRandomLocationinNavigableRadius (Transformation|GetWorldLocation _spawnsphere) (Components|Sphere|GetScaledSphereRadius _spawnsphere) 0 0))
  (if (> (Math|Vector|Distance(Vector) _randomlocation (Transformation|GetWorldLocation _blocksphere)) (Variables|/Script/Engine.SphereComponent|GetSphereRadius _blocksphere))
    (Game|SpawnActorfromClass "/Game/Blueprint/BP_Boss.BP_Boss_C" (Math|Transform|MakeTransform _randomlocation "0, 0, 0" "1,1,1") "Undefined" 0 0)
    (bind _returnvalue (Utilities|GetDataTableRow "/Game/Blueprint/Stats_DataTable.Stats_DataTable" "BossSpawnRate")
      (:then
        (Utilities|FlowControl|Delay (Utilities|SpawnRateMath (.value _returnvalue))) ; Spawn Time
        (CallFunction|SpawnBoss)))
    (else
      (CallFunction|SpawnBoss))))

(event Custom|SpawnGoblin
  (bind _blocksphere (Variables|Default|GetBlockSphere))
  (bind _spawnsphere (Variables|Default|GetSpawnSphere))
  ;[1 1 1] SPawn Boss units
  (bind _randomlocation (Class|NavigationSystemV1|GetRandomLocationinNavigableRadius (Transformation|GetWorldLocation _spawnsphere) (Components|Sphere|GetScaledSphereRadius _spawnsphere) 0 0))
  (if (> (Math|Vector|Distance(Vector) _randomlocation (Transformation|GetWorldLocation _blocksphere)) (Variables|/Script/Engine.SphereComponent|GetSphereRadius _blocksphere))
    (Game|SpawnActorfromClass "/Game/Blueprint/BP_Goblin.BP_Goblin_C" (Math|Transform|MakeTransform _randomlocation "0, 0, 0" "1,1,1") "Undefined" 0 0)
    (bind _returnvalue (Utilities|GetDataTableRow "/Game/Blueprint/Stats_DataTable.Stats_DataTable" "GolbinSpawnRate")
      (:then
        (Utilities|FlowControl|Delay (.value _returnvalue)) ; Spawn Time
        (CallFunction|SpawnGoblin)))
    (else
      (CallFunction|SpawnGoblin))))

(event Custom|SpawnElite
  (bind _blocksphere (Variables|Default|GetBlockSphere))
  (bind _spawnsphere (Variables|Default|GetSpawnSphere))
  ;[1 1 1] SPawn Elite units
  (bind _randomlocation (Class|NavigationSystemV1|GetRandomLocationinNavigableRadius (Transformation|GetWorldLocation _spawnsphere) (Components|Sphere|GetScaledSphereRadius _spawnsphere) 0 0))
  (if (> (Math|Vector|Distance(Vector) _randomlocation (Transformation|GetWorldLocation _blocksphere)) (Variables|/Script/Engine.SphereComponent|GetSphereRadius _blocksphere))
    (Game|SpawnActorfromClass "/Game/Blueprint/BP_EliteTank.BP_EliteTank_C" (Math|Transform|MakeTransform _randomlocation "0, 0, 0" "1,1,1") "Undefined" 0 0)
    (bind _returnvalue (Utilities|GetDataTableRow "/Game/Blueprint/Stats_DataTable.Stats_DataTable" "EliteSpawnRate")
      (:then
        (Utilities|FlowControl|Delay (Utilities|SpawnRateMath (.value _returnvalue))) ; Spawn Time
        (CallFunction|SpawnElite)))
    (else
      (CallFunction|SpawnElite))))

(event EventBeginPlay
  (Audio|PlaySoundatLocation "/Game/Ultimate_SFX_Bundle/Horror_SFX_Bundle/Impacts_Sweeps/Wavs/Impact_Samurai_03.Impact_Samurai_03" "0, 0, 0" "0, 0, 0" 1.0 1.0 0.0 0 0 0) ; Sound at start
  (CallFunction|SpawnUnit)
  (Utilities|FlowControl|Sequence
    (:then_0
      ;[1 1 1] Spawn Elite after delay at start
      (bind _returnvalue (Utilities|GetDataTableRow "/Game/Blueprint/Stats_DataTable.Stats_DataTable" "EliteSpawnRate")
        (:then
          (Utilities|FlowControl|Delay (.value _returnvalue)) ; Spawn Time
          (CallFunction|SpawnElite))))
    (:then_1
      ;[1 1 1] SPawn boss after delay at start
      (bind _returnvalue_2 (Utilities|GetDataTableRow "/Game/Blueprint/Stats_DataTable.Stats_DataTable" "BossSpawnRate")
        (:then
          (Utilities|FlowControl|Delay (.value _returnvalue_2)) ; Spawn Time
          (CallFunction|SpawnBoss))))
    (:then_2
      ;[1 1 1] Spawn Goblin
      (bind _returnvalue_3 (Utilities|GetDataTableRow "/Game/Blueprint/Stats_DataTable.Stats_DataTable" "GolbinSpawnRate")
        (:then
          (Utilities|FlowControl|Delay (.value _returnvalue_3)) ; Spawn Time
          (CallFunction|SpawnGoblin))))))

(fn ConstructionScript
  (bind _returnvalue (Utilities|GetDataTableRow "/Game/Blueprint/Stats_DataTable.Stats_DataTable" "SPawnRateIncreaseRate")
    (:then
      (Variables|Default|SetDifficultyIncreaseRate (.value _returnvalue))
      (bind _returnvalue_2 (Utilities|GetDataTableRow "/Game/Blueprint/Stats_DataTable.Stats_DataTable" "SpawnRateDividerIncreaseAmount")
        (:then
          (Variables|Default|SetSpawnRateIncrement (.value _returnvalue_2))
          (bind _returnvalue_3 (Utilities|GetDataTableRow "/Game/Blueprint/Stats_DataTable.Stats_DataTable" "SpawnRateDividerCap")
            (:then
              (Variables|Default|SetSpawnRateDividerCap (.value _returnvalue_3)))))))))