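; Base game mode that manages the save game and starts play.
; On BeginPlay it disables screen messages, then loads the save slot and reapplies its volume, or creates a new save.
; SaveVolume and SaveBest write volume and score asynchronously, with volume applied through a sound mix class override.
; StartGame spawns and possesses the pawn at the PlayerStart, triggers the spawner and lowers the ambient wind sound.
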(event Custom|SaveVolume
  (params (Volume :type Float%20%28single-precision%29))
  ;[1 1 1] Save
  (bind _output_get (Variables|/Game/Blueprint/BP_SaveGame.BP_SaveGame_C|SetVolume (Variables|Default|GetSaveInstance) Volume))
  (|AsyncSaveGametoSlot (Variables|Default|GetSaveInstance) (Variables|Default|GetSaveSlot)
    (:then
      (Audio|SetSoundMixClassOverride "/Game/Ultimate_SFX_Bundle/SoundMix.SoundMix" "/Engine/EngineSounds/Master.Master" _output_get 1.0 1.0 true) ; Set Volume
    )))

(event Custom|SaveBest
  (params (Score :type Integer))
  ;[1 1 1] Save
  (Variables|/Game/Blueprint/BP_SaveGame.BP_SaveGame_C|SetScore (Variables|Default|GetSaveInstance) Score)
  (|AsyncSaveGametoSlot (Variables|Default|GetSaveInstance) (Variables|Default|GetSaveSlot)))

(event EventBeginPlay
  (bind _saveslot (Variables|Default|GetSaveSlot))
  (Development|ExecuteConsoleCommand "DISABLEALLSCREENMESSAGES" 0)
  ;[1 1 1] Load
  (bind _returnvalue (SaveGame|LoadGamefromSlot _saveslot))
  (Utilities|IsValid _returnvalue
    (:Is%20Valid
      (bind _asbp_save_game (Utilities|Casting|CastToBP_SaveGame _returnvalue))
      (bind _output_get (Variables|Default|SetSaveInstance _asbp_save_game))
      (CallFunction|SaveVolume (Variables|/Game/Blueprint/BP_SaveGame.BP_SaveGame_C|GetVolume _output_get)))
    (:Is%20Not%20Valid
      (bind _returnvalue_2 (SaveGame|CreateSaveGameObject "/Game/Blueprint/BP_SaveGame.BP_SaveGame_C"))
      (bind _output_get_2 (Variables|Default|SetSaveInstance _returnvalue_2))
      (|AsyncSaveGametoSlot _output_get_2 _saveslot))))

(fn ConstructionScript)

(fn StartGame
  (bind _returnvalue (Game|GetPlayerController 0))
  (bind _returnvalue_2 (Actor|GetActorOfClass "/Script/Engine.PlayerStart"))
  (Utilities|IsValid _returnvalue_2
    (:Is%20Valid
      (bind _returnvalue_3 (Game|SpawnActorfromClass "/Game/Blueprint/BP_BasePawn.BP_BasePawn_C" (Transformation|GetActorTransform _returnvalue_2) "Undefined" 0 0))
      (Pawn|UnPossess _returnvalue)
      (Pawn|Possess _returnvalue _returnvalue_3)
      (bind _returnvalue_4 (Actor|GetActorOfClass "/Game/Blueprint/BP_BaseSpawner.BP_BaseSpawner_C"))
      (Default|StartSpawning _returnvalue_4)
      ;[1 1 1] For the ambient sound of wind
      (bind _outactors (Actor|GetAllActorsOfClass "/Script/Engine.AmbientSound"))
      (for _array_element _outactors
        (if (Utilities|Enum|Equal(Enum) (Utilities|GetDisplayName _array_element) "AmbientSound")
          (Audio|Components|Audio|SetVolumeMultiplier (Variables|/Script/Engine.AmbientSound|GetAudioComponent _array_element) 0.05 :!class /Script/Engine.AudioComponent))))))