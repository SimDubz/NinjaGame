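; BP_EliteTank is the elite variant of a tank character, with boosted health, a score multiplier and a random ability pickup drop.
; The construction script sets large-monster death sounds and reads the elite score multiplier from the stats DataTable.
; BaseHealthMath scales the parent's result by the table's elite health multiplier.
; LogicOnDestroy spawns BP_AbilityPickup_Random at the mesh location before running the parent logic.
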(event EventBeginPlay
  (|CallParentFunction) ; This node is disabled and will not be called.\nDrag off pins to build functionality.
)

(event Collision|EventActorBeginOverlap
  (params (OtherActor :type Actor%20Object%20Reference)))

(event EventTick
  (params (DeltaSeconds :type Float%20%28single-precision%29)))

(fn ConstructionScript
  (|CallParentFunction)
  (Variables|Default|SetDeathSounds (Utilities|Array|MakeArray "/Game/Ultimate_SFX_Bundle/Monster_Sounds_Pro/Wavs/large_monster_attack/large_monster_attack_1.large_monster_attack_1" "/Game/Ultimate_SFX_Bundle/Monster_Sounds_Pro/Wavs/large_monster_attack/large_monster_attack_2.large_monster_attack_2" "/Game/Ultimate_SFX_Bundle/Monster_Sounds_Pro/Wavs/large_monster_attack/large_monster_attack_3.large_monster_attack_3" "/Game/Ultimate_SFX_Bundle/Monster_Sounds_Pro/Wavs/large_monster_attack/large_monster_attack_4.large_monster_attack_4" "/Game/Ultimate_SFX_Bundle/Monster_Sounds_Pro/Wavs/large_monster_attack/large_monster_attack_5.large_monster_attack_5"))
  (bind _returnvalue (Utilities|GetDataTableRow "/Game/Blueprint/Stats_DataTable.Stats_DataTable" "EliteScoreMultiplier")
    (:then
      (Variables|Default|SetScoreMultiplier (.value _returnvalue)))))

(fn LogiconDestroy
  ;[1 1 1] Spawn Ability pickup randomly
  (Game|SpawnActorfromClass "/Game/Blueprint/AltShurikens/BP_AbilityPickup_Random.BP_AbilityPickup_Random_C" (Math|Transform|MakeTransform (Transformation|GetWorldLocation (Variables|Character|GetMesh)) "0, 0, 0" "1,1,1") "Undefined" 0 0)
  (|CallParentFunction)
  (return))

(fn BaseHealthMath
  (bind _returnvalue (|CallParentFunction))
  (bind _returnvalue_2 (Utilities|GetDataTableRow "/Game/Blueprint/Stats_DataTable.Stats_DataTable" "EliteHealthMultiplier")
    (:then
      (return (* _returnvalue (.value _returnvalue_2))))))